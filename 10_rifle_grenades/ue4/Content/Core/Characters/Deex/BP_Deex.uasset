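; BP_Deex is the Blueprint for the Deex character, adding a fire effect that shows while the character slides.
; Tick polls the movement component's sliding state to toggle the Fire component's visibility, which BeginPlay initially hides.
; Sprint start and stop events only call their parent versions.
; An old timeline that lerps spring arm length for sprinting remains disconnected and never runs.
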(event EventOnSprintStarted
  (|CallParentFunction))

(event EventOnSprintStopped
  (|CallParentFunction))

(event EventBeginPlay
  (Rendering|SetVisibility (Variables|Default|GetFire) false false))

(event EventTick
  (params (DeltaSeconds :type Float%20%28single-precision%29))
  (bind _fire (Variables|Default|GetFire))
  ;[1 1 1] ass fire on sliding
  (bind _returnvalue (Class|BaseMovementComponent|IsSliding (Class|BaseCharacter|GetMoveComp)))
  (if _returnvalue
    (Rendering|SetVisibility _fire true false)
    (else
      (Rendering|SetVisibility _fire false false))))

(fn ConstructionScript)